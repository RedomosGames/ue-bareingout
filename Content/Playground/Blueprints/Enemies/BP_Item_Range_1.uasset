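; BP_Item_Range_1 is an explosive projectile, filed under Enemies, that deals area damage on impact.
; It sets its ProjectileMovement velocity from a variable at BeginPlay.
; On collision it spawns a scaled explosion effect, runs a sphere trace meant to find the player, then destroys itself.
; The trace sends a damage message with a negative amount to the single hit actor and leaves debug drawing on.
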(event OnComponentHit(ProjectileCollision)
  (params (HitComponent :type Primitive%20Component%20Object%20Reference) (OtherActor :type Actor%20Object%20Reference) (OtherComp :type Primitive%20Component%20Object%20Reference) (NormalImpulse :type Vector :default "0, 0, 0") (Hit :type Hit%20Result%20Structure%20%28by%20ref%29))
  ;[0 1 0 0.5] On Hit, call Trace and destroy
  (Niagara|SpawnSystematLocation "/Game/LowPolyVFX/Particles/P_Ems_Explosion_01_Converted.P_Ems_Explosion_01_Converted" (Transformation|GetActorLocation) "0, 0, 0" "4.000000,4.000000,4.000000")
  (CallFunction|ImpactTrace)
  (Actor|DestroyActor))

(event Custom|ImpactTrace
  (bind _returnvalue (Transformation|GetActorLocation))
  ;[0 1 0 0.5] Do a trace for the player on impact
  (bind (_outhit _returnvalue_2) (Collision|SphereTraceForObjects _returnvalue _returnvalue 2e+02 (Utilities|Array|MakeArray "ObjectTypeQuery7") false 0 "ForDuration"))
  (if _returnvalue_2
    (Class|BPIDamageable|TakeDamage(Message) (.HitActor (Collision|BreakHitResult _outhit)) (Utilities|Struct|MakeS_DamageInfo -1e+01 "NewEnumerator0") self)))

(event EventBeginPlay
  ;[0 1 1 0.5] Set Projectile Velocity
  (Variables|/Script/Engine.MovementComponent|SetVelocity (Variables|Default|GetProjectileMovement) (Variables|Default|GetVelocity)))

(fn ConstructionScript)