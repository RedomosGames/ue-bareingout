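; BP_Dummy is a test dummy enemy in the Playground that reports its damage handling through debug prints.
; TakeDamage forwards damage info to DamageComponent and returns its result, while the component's death, blocked and damage response events each print a message.
; Every tick it also prints a float attribute read from its Ability System Component, labeled as health.
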(event OnDeath(DamageComponent)
  ;[0 1 0 0.5] Damage Comp
  (Development|PrintString "Dead"))

(event OnBlocked(DamageComponent)
  (params (CanBeParried :type Boolean))
  ;[0 1 0 0.5] Damage Comp
  (Development|PrintString "Blocked"))

(event OnDamageResponse(DamageComponent)
  (params (DamageResponse :type E_DamageResponse%20Enum :default "NewEnumerator0"))
  ;[0 1 0 0.5] Damage Comp
  (Development|PrintString (Utilities|String|EnumtoString DamageResponse)))

(event EventTick
  (params (DeltaSeconds :type Float%20%28single-precision%29))
  ;[1 0 1 0.5] Print Health
  (Development|PrintString (Utilities|String|ToString(Float) (.ReturnValue (Ability|Attribute|GetFloatAttributefromAbilitySystemComponent (Ability|GetAbilitySystemComponent 0) "(AttributeName=\"Health\",Attribute=/Script/Playground.BasicAttributeSet:Health,AttributeOwner=\"/Script/CoreUObject.Class'/Script/Playground.BasicAttributeSet'\")"))) true true "(R=1.000000,G=0.004322,B=0.021989,A=1.000000)" 0.0))

(fn ConstructionScript)

(fn TakeDamage
  (params (DamageInfo :type S%20Damage%20Info%20Structure))
  (bind _wasdamaged (Default|TakeDamage (Variables|Default|GetDamageComponent) DamageInfo))
  (return _wasdamaged))