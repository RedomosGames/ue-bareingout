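; Melee enemy Blueprint that attacks with a montage and can block incoming player hits.
; Attack runs a right-hand CombatComponent trace for blockable, parryable damage during the montage, ending on completion or interruption.
; TakeDamage rolls BlockChance for blockable hits, gated by the player's pursuit check, before forwarding to DamageComponent.
; Blocking halts movement and starts a hold timer; a blocked hit clears it and plays a reaction montage before ending the block.
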(event OnBlocked(DamageComponent)
  (params (CanBeParried :type Boolean) (DamageCauser :type Actor%20Object%20Reference))
  ;[0 1 0 0.5] Block Player Attack
  (Variables|Default|SetIsReactingToBlock true)
  (Utilities|Time|ClearandInvalidateTimerbyHandle (Variables|Default|GetHoldBlockTimer))
  (Animation|Montage|PlayMontage (Variables|Character|GetMesh) "/Game/Imports/Animations/UAL2_StandardSword_Regular_A_Rec2_Montage.UAL2_StandardSword_Regular_A_Rec2_Montage"
    (:OnCompleted
      _)
    (:OnInterrupted
      _))
  (CallFunction|EndBlock))

(event Custom|StartBlock
  ;[0 1 0 0.5] Block Player Attack
  (Utilities|Time|ClearandInvalidateTimerbyHandle (Variables|Default|GetHoldBlockTimer))
  (Components|Movement|StopMovementImmediately (Variables|Character|GetCharacterMovement))
  (Variables|/Game/Playground/Blueprints/Components/DamageComponent.DamageComponent_C|SetIsBlocking (Variables|Default|GetDamageComponent) true)
  (bind _returnvalue (Utilities|Time|SetTimerbyEvent (EventDispatchers|CreateEvent :!event Custom|EndBlock) 2.0))
  (Variables|Default|SetHoldBlockTimer _returnvalue))

(event Custom|EndBlock
  ;[0 1 0 0.5] Block Player Attack
  (Variables|/Game/Playground/Blueprints/Components/DamageComponent.DamageComponent_C|SetIsBlocking (Variables|Default|GetDamageComponent) false)
  (Variables|Default|SetIsReactingToBlock false)
  (Default|CallOnBlockEnded))

(event EventBeginPlay
  (|CallParentFunction) ; This node is disabled and will not be called.\nDrag off pins to build functionality.
)

(event Collision|EventActorBeginOverlap
  (params (OtherActor :type Actor%20Object%20Reference)))

(event EventTick
  (params (DeltaSeconds :type Float%20%28single-precision%29))
  (|CallParentFunction DeltaSeconds) ; This node is disabled and will not be called.\nDrag off pins to build functionality.
)

(event EventAttack
  (params (AttackTarget :type Actor%20Object%20Reference))
  (bind _combatcomponent (Variables|Default|GetCombatComponent))
  (|CallParentFunction AttackTarget)
  (Animation|Montage|PlayMontage (Variables|Character|GetMesh) "/Game/Characters/Mannequins/Anims/Unarmed/Attack/AM_Attack_1.AM_Attack_1"
    (:then
      (Default|StartTrace _combatcomponent false true false false (Utilities|Struct|MakeS_DamageInfo -1e+01 "NewEnumerator1" false true true) false))
    (:OnCompleted
      (CallFunction|AttackEnd AttackTarget :!label _label)
      (Default|EndTrace _combatcomponent))
    (:OnInterrupted
      (goto _label))))

(fn ConstructionScript
  (|CallParentFunction))

(fn TakeDamage
  (params (DamageInfo :type S%20Damage%20Info%20Structure) (Damager :type Actor%20Object%20Reference))
  (if (Utilities|Struct|BreakS_DamageInfo DamageInfo)
    (CallFunction|TrytoBlock))
  (bind _wasdamaged (Default|TakeDamage (Variables|Default|GetDamageComponent) DamageInfo Damager))
  (return _wasdamaged))

(fn TrytoBlock
  (bind _inpursuit (Class|BPIPursuit|CheckIsinPursuit(Message) (Game|GetPlayerCharacter 0)))
  (if (and (<= (Math|Random|RandomFloat) (Variables|Default|GetBlockChance)) _inpursuit)
    (CallFunction|StartBlock)))