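; BP_EnemyManager keeps the playground stocked with melee enemies, up to a set spawn amount.
; A looping timer spawns one inside a random box under SpawnCollisionFolder when a randomly picked area is far enough from the player.
; The distance check and spawn location draw separate random picks, so they can use different boxes.
; It registers with GS_Playground's enemy death callback to remove dead enemies from its tracked list.
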(event Custom|GetRandomPointInSpawnAreas
  (bind _spawncollisionfolder (Variables|Default|GetSpawnCollisionFolder))
  (bind _children (Components|GetChildrenComponents _spawncollisionfolder false))
  (bind _outitem (Utilities|Array|Random _children))
  (if (< (Utilities|Array|Length (Variables|Default|GetEnemiesSpawned)) (Variables|Default|GetEnemySpawnAmount))
    (if (> (Math|Vector|Distance(Vector) (Transformation|GetWorldLocation _outitem) (Transformation|GetActorLocation (Game|GetPlayerCharacter 0))) 1.5e+03)
      (bind _asbox_collision (Utilities|Casting|CastToBoxComponent _outitem))
      (bind _returnvalue (Game|SpawnActorfromClass "/Game/Playground/Blueprints/Enemies/BP_Enemy_Melee_1.BP_Enemy_Melee_1_C" (Math|Transform|MakeTransform (Math|Random|RandomPointinBoundingBox (Transformation|GetWorldLocation _asbox_collision) (Variables|/Script/Engine.BoxComponent|GetBoxExtent _asbox_collision)) "0, 0, 0" "1.000000,1.000000,1.000000") "Undefined" "MultiplyWithRoot" 0 0))
      (Utilities|Array|AddUnique (Variables|Default|GetEnemiesSpawned) _returnvalue)
      (else
        (Development|PrintString "to Close To Spawn")))))

(event Custom|FinishOnEnemyDeath
  (params (EnemyRef :type BP%20Enemy%20Base%20Object%20Reference))
  (Utilities|Array|RemoveItem (Variables|Default|GetEnemiesSpawned) EnemyRef))

(event EventBeginPlay
  (Utilities|Time|SetTimerbyFunctionName 0 "GetRandomPointInSpawnAreas" 1.0 true)
  (bind _asgs_playground (Utilities|Casting|CastToGS_Playground (Game|GetGameState)))
  (EventDispatchers|AssignOnEnemyDeath _asgs_playground (delegate Custom|FinishOnEnemyDeath)))

(fn ConstructionScript)