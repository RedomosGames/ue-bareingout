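; Base enemy character that plays montages on noticing or losing the player, jumps by projectile arc and exposes patrol, range, speed and health to AI.
; DamageComponent events drive hit, stun, knockback and death reactions, switching AIC_Enemy_Base states and flashing the material.
; Attacks reserve tokens from their target, tracked per target and returned on attack end or death.
; Knockback fires a gameplay event, packing strength and duration into a HitResult.
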(event OnDeath(DamageComponent)
  (bind _reserveattacktokens (Variables|Default|GetReserveAttackTokens))
  (bind _aicontrollerref (Variables|Default|GetAiControllerRef))
  ;[0 1 0 0.5] Damage Comp
  (Default|SetStateasDead _aicontrollerref)
  (AI|Logic|StopLogic (Variables|/Script/AIModule.AIController|GetBrainComponent _aicontrollerref) "")
  (bind _notifyname (Animation|Montage|PlayMontage (Variables|Character|GetMesh) "/Game/Imports/Animations/UAL1_StandardDeath01_Montage.UAL1_StandardDeath01_Montage")
    (:then
      (Audio|PlaySoundatLocation "/Game/Imports/sounds/Death.death" (Transformation|GetActorLocation) "0, 0, 0" 1.0 1.0 0.0 0 0 0 0)
      (Variables|/Game/Playground/Blueprints/Components/DamageComponent.DamageComponent_C|SetIsDead (Variables|Default|GetDamageComponent) true)
      (bind _keys (Utilities|Map|Keys _reserveattacktokens))
      (for _array_element _keys
        (Class|BPIDamageable|ReturnAttackToken(Message) _array_element (.Value (Utilities|Map|Find _reserveattacktokens _array_element)))))
    (:OnNotifyBegin
      (switch name _notifyname
        (:Death
          (Actor|DestroyActor))))))

(event OnBlocked(DamageComponent)
  (params (CanBeParried :type Boolean) (DamageCauser :type Actor%20Object%20Reference))
  ;[0 1 0 0.5] Damage Comp
  (Development|PrintString "Blocked"))

(event OnDamageResponse(DamageComponent)
  (params (DamageResponse :type E_DamageResponse%20Enum :default "NewEnumerator0") (DamageCauser :type Actor%20Object%20Reference))
  ;[0 1 0 0.5] Damage Comp
  (bind _returnvalue (Utilities|Time|SetTimerbyEvent (delegate Custom|FlashHitReaction) 0.15 true))
  (Default|SetStateasFrozen (Variables|Default|GetAiControllerRef))
  (switch Utilities|FlowControl|Switch|SwitchonE_DamageResponse DamageResponse
    (:NewEnumerator1
      (CallFunction|ApplyKnockback 525.0 0.15)
      (Animation|Montage|PlayMontage (Variables|Character|GetMesh) "/Game/Imports/Animations/UAL1_StandardHit_Chest1_Montage.UAL1_StandardHit_Chest1_Montage"
        (:then
          (Audio|PlaySoundatLocation "/Game/Imports/sounds/hit.hit" (Transformation|GetActorLocation) "0, 0, 0" 1.0 1.0 0.0 0 0 0 0))
        (:OnCompleted
          (Default|SetStateasAttacking (Variables|Default|GetAiControllerRef) DamageCauser true :!label _label))
        (:OnInterrupted
          (goto _label))))
    (:NewEnumerator3
      (CallFunction|ApplyKnockback 6.5e+02 0.18)
      (Animation|Montage|PlayMontage (Variables|Character|GetMesh) "/Game/Imports/Animations/UAL1_StandardHit_Chest1_Montage.UAL1_StandardHit_Chest1_Montage"
        (:then
          (Audio|PlaySoundatLocation "/Game/Imports/sounds/stunner.stunner" (Transformation|GetActorLocation) "0, 0, 0" 1.0 1.0 0.0 0 0 0 0)
          (Variables|/Game/Playground/Blueprints/Components/DamageComponent.DamageComponent_C|SetIsStunned (Variables|Default|GetDamageComponent) true)
          (Utilities|FlowControl|RetriggerableDelay 2.0)
          (Variables|/Game/Playground/Blueprints/Components/DamageComponent.DamageComponent_C|SetIsStunned (Variables|Default|GetDamageComponent) false)
          (Default|SetStateasAttacking (Variables|Default|GetAiControllerRef) DamageCauser true))))
    (:NewEnumerator4
      (CallFunction|ApplyKnockback 1e+03 0.25)
      (Animation|Montage|PlayMontage (Variables|Character|GetMesh) "/Game/Imports/Animations/UAL2_StandardHit_Knockback1_Montage.UAL2_StandardHit_Knockback1_Montage"
        (:then
          (Audio|PlaySoundatLocation "/Game/Imports/sounds/knockback_APYIqoJr.knockback_APYIqoJr" (Transformation|GetActorLocation) "0, 0, 0" 1.0 1.0 0.0 0 0 0 0)
          (Variables|/Game/Playground/Blueprints/Components/DamageComponent.DamageComponent_C|SetIsInteruptable (Variables|Default|GetDamageComponent) false))
        (:OnCompleted
          (Animation|Montage|PlayMontage (Variables|Character|GetMesh) "/Game/Imports/Animations/UAL2_StandardLayToIdle1_Montage.UAL2_StandardLayToIdle1_Montage"
            (:OnCompleted
              _)
            (:OnInterrupted
              _))
          (Variables|/Game/Playground/Blueprints/Components/DamageComponent.DamageComponent_C|SetIsInteruptable (Variables|Default|GetDamageComponent) true)
          (Default|SetStateasAttacking (Variables|Default|GetAiControllerRef) DamageCauser true))))))

(event Custom|FlashHitReaction
  ;[0 1 0 0.5] Damage Comp
  (Utilities|FlowControl|FlipFlop
    (:A
      (Rendering|Material|SetMaterial (Variables|Character|GetMesh) 0 "/Game/Playground/Materials/M_FlashHitReaction.M_FlashHitReaction"))
    (:B
      (Rendering|Material|SetMaterial (Variables|Character|GetMesh) 0 "/Game/Imports/SkeletalMesh/Banana/skin.skin")
      (Utilities|Time|ClearandInvalidateTimerbyHandle (stale OnDamageResponse(DamageComponent) _returnvalue)))))

(event EventEndPlay
  (params (EndPlayReason :type EEndPlayReason%20Enum :default "Destroyed"))
  (bind _damagecomponent (Variables|Default|GetDamageComponent))
  ;[0 1 1 0.5] End Play
  (EventDispatchers|UnbindallEventsfromOnBlocked _damagecomponent)
  (EventDispatchers|UnbindallEventsfromOnDamageResponse _damagecomponent)
  (EventDispatchers|UnbindallEventsfromOnDeath _damagecomponent))

(event EventTick
  (params (DeltaSeconds :type Float%20%28single-precision%29))
  ;[1 0 1 0.5] Print Health
  (Development|PrintString (Utilities|String|ToString(Float) (.ReturnValue (Ability|Attribute|GetFloatAttributefromAbilitySystemComponent (Ability|GetAbilitySystemComponent 0) "(AttributeName=\"Health\",Attribute=/Script/Playground.BasicAttributeSet:Health,AttributeOwner=\"/Script/CoreUObject.Class'/Script/Playground.BasicAttributeSet'\")"))) true true "(R=1.000000,G=0.004322,B=0.021989,A=1.000000)" 0.0))

(event EventBeginPlay
  ;[0 1 1 0.5] Begin Play
  (bind _asaic_enemy_base (Utilities|Casting|CastToAIC_Enemy_Base (AI|GetAIController self)))
  (Variables|Default|SetAiControllerRef _asaic_enemy_base))

(event EventLostPlayer
  (Variables|editables|SetDidNoticePlayer false)
  (Animation|Montage|PlayMontage (Variables|Character|GetMesh) "/Game/Imports/Animations/UAL1_StandardDance_Loop1_Montage.UAL1_StandardDance_Loop1_Montage"
    (:OnCompleted
      _)
    (:OnInterrupted
      _))
  (Default|CallOnLostPlayer))

(event EventNoticePlayer
  (Variables|editables|SetDidNoticePlayer true)
  (Animation|Montage|PlayMontage (Variables|Character|GetMesh) "/Game/Imports/Animations/UAL1_StandardInteract1_Montage.UAL1_StandardInteract1_Montage"
    (:OnCompleted
      _)
    (:OnInterrupted
      _))
  (Default|CallOnNoticePlayer))

(event EventJumptoDestination
  (params (Destination :type Vector :default "0, 0, 0"))
  (bind (_x _y _z) (Math|Vector|BreakVector Destination))
  (bind _outlaunchvelocity (Game|SuggestProjectileVelocityCustomArc (Transformation|GetActorLocation) (Math|Vector|MakeVector _x _y (+ _z 1.5e+02)) 0.0 0.5))
  (Character|LaunchCharacter _outlaunchvelocity true true))

(event EventReturnAttackToken
  (params (Amount :type Integer))
  (Default|ReturnAttackToken (Variables|Default|GetDamageComponent) Amount))

(event EventStoreAttackTokens
  (params (AttackTarget :type Actor%20Object%20Reference) (Amount :type Integer))
  (bind _reserveattacktokens (Variables|Default|GetReserveAttackTokens))
  (bind (_value _returnvalue) (Utilities|Map|Find _reserveattacktokens AttackTarget))
  (Utilities|Map|Add (Variables|Default|GetReserveAttackTokens) AttackTarget (select _returnvalue (+ Amount _value) Amount)))

(event EventAttackEnd
  (params (AttackTarget :type Actor%20Object%20Reference))
  (bind _tokensusedincurretnattack (Variables|Default|GetTokensUsedInCurretnAttack))
  (Class|BPIDamageable|ReturnAttackToken(Message) AttackTarget _tokensusedincurretnattack)
  (CallFunction|StoreAttackTokens AttackTarget (* _tokensusedincurretnattack -1))
  (Default|CallOnAttackEnd))

(fn ConstructionScript)

(fn ApplyKnockback
  (params (Strength :type Float%20%28single-precision%29) (Duration :type Float%20%28single-precision%29))
  (Ability|SendGameplayEventtoActor self "(TagName=\"Event.Combat.Knockback\")" (Utilities|Struct|MakeGameplayEventData (Ability|TargetData|AbilityTargetDatafromHitResult (Collision|MakeHitResult false false Duration Strength "0, 0, 0" "0, 0, 0" "0,0,1" "0,0,1" 0 0))))
  (return))

(fn AttackStart
  (params (AttackTarget :type Actor%20Object%20Reference) (TokensNeeded :type Integer))
  (bind _success (Class|BPIDamageable|ReserveAttackToken(Message) AttackTarget TokensNeeded))
  (if _success
    (CallFunction|StoreAttackTokens AttackTarget TokensNeeded)
    (Variables|Default|SetTokensUsedInCurretnAttack TokensNeeded)
    (return true)
    (else
      (return false))))

(fn GetCurrentHealth
  (return (.ReturnValue (Ability|Attribute|GetFloatAttributefromAbilitySystemComponent (Ability|GetAbilitySystemComponent 0) "(AttributeName=\"Health\",Attribute=/Script/Playground.BasicAttributeSet:Health,AttributeOwner=\"/Script/CoreUObject.Class'/Script/Playground.BasicAttributeSet'\")"))))

(fn GetIdealRange
  (return 125.0 5e+02))

(fn GetMaxHealth
  (return (.ReturnValue (Ability|Attribute|GetFloatAttributefromAbilitySystemComponent (Ability|GetAbilitySystemComponent 0) "(AttributeName=\"MaxHealth\",Attribute=/Script/Playground.BasicAttributeSet:MaxHealth,AttributeOwner=\"/Script/CoreUObject.Class'/Script/Playground.BasicAttributeSet'\")"))))

(fn GetPatrolRoute
  (return (Variables|Editables|GetPatrolRoute)))

(fn IsAttacking
  (return (Variables|/Game/Playground/Blueprints/Components/DamageComponent.DamageComponent_C|GetIsAttacking (Variables|Default|GetDamageComponent))))

(fn IsDead
  (return (Variables|/Game/Playground/Blueprints/Components/DamageComponent.DamageComponent_C|GetIsDead (Variables|Default|GetDamageComponent))))

(fn ReserveAttackToken
  (params (Amount :type Integer))
  (bind _sucess (Default|ReserveAttackToken (Variables|Default|GetDamageComponent) Amount))
  (return _sucess))

(fn SetMovementSpeed
  (params (Speed :type E_MovementSpeed%20Enum :default "NewEnumerator0"))
  (bind _output_get (Variables|/Script/Engine.CharacterMovementComponent|SetMaxWalkSpeed (Variables|Character|GetCharacterMovement) (Utilities|Select :Index Speed :NewEnumerator0 0.0 :NewEnumerator1 2e+02 :NewEnumerator2 4e+02 :NewEnumerator3 6e+02)))
  (return _output_get))

(fn TakeDamage
  (params (DamageInfo :type S%20Damage%20Info%20Structure) (Damager :type Actor%20Object%20Reference))
  (bind _wasdamaged (Default|TakeDamage (Variables|Default|GetDamageComponent) DamageInfo Damager))
  (return _wasdamaged))