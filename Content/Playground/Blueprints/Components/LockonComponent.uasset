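; Lock-on component that toggles the player camera and character facing onto a nearby target.
; A sphere trace around the owner picks the target, then look input is ignored, the spring arm is raised and movement follows controller rotation.
; A looping timer aims control rotation at the target and ends lock-on when it becomes invalid.
; ChangeTarget repeats the trace, switching only if the single hit is a different actor.
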(event Custom|ChangeTarget
  (bind _returnvalue (Components|GetOwner))
  (bind _returnvalue_2 (Transformation|GetActorLocation _returnvalue))
  ;[0 1 0 0.5] Change Target
  (if (Variables|Default|GetIsLockedon)
    (bind (_outhit _returnvalue_3) (Collision|SphereTraceForObjects _returnvalue_2 _returnvalue_2 (Variables|Default|GetLockonRadius) (Utilities|Array|MakeArray "ObjectTypeQuery8") false 0 "ForDuration" true "(R=1.000000,G=0.000000,B=0.000000,A=1.000000)" "(R=0.000000,G=1.000000,B=0.000000,A=1.000000)" 1.0))
    (if _returnvalue_3
      (if (not (== (.HitActor (Collision|BreakHitResult _outhit)) (Variables|Default|GetLockonTarget)))
        (Variables|Default|SetLockonTarget (.HitActor (Collision|BreakHitResult _outhit)))))))

(event Custom|StartLockon
  (bind _returnvalue (Game|GetPlayerCharacter 0))
  (bind _returnvalue_2 (Components|GetOwner))
  (bind _returnvalue_3 (Transformation|GetActorLocation _returnvalue_2))
  (bind _charactermovement (Variables|/Script/Engine.Character|GetCharacterMovement _returnvalue))
  ;[0 1 0 0.5] Start Lockon
  (bind (_outhit _returnvalue_4) (Collision|SphereTraceForObjects _returnvalue_3 _returnvalue_3 (Variables|Default|GetLockonRadius) (Utilities|Array|MakeArray "ObjectTypeQuery8") false 0 "ForDuration" true "(R=1.000000,G=0.000000,B=0.000000,A=1.000000)" "(R=0.000000,G=1.000000,B=0.000000,A=1.000000)" 1.0))
  (if _returnvalue_4
    (Variables|Default|SetLockonTarget (.HitActor (Collision|BreakHitResult _outhit)))
    (Input|SetIgnoreLookInput (Game|GetPlayerController 0) true)
    (Variables|Default|SetIsLockedon true)
    (Variables|/Script/Engine.SpringArmComponent|SetTargetOffset (Actor|GetComponentbyClass (Components|GetOwner) "/Script/Engine.SpringArmComponent") "0.000000,0.000000,100.000000")
    (Variables|/Script/Engine.CharacterMovementComponent|SetbOrientRotationToMovement _charactermovement false)
    (Variables|/Script/Engine.CharacterMovementComponent|SetbUseControllerDesiredRotation _charactermovement true)
    (bind _returnvalue_5 (Utilities|Time|SetTimerbyEvent (delegate Custom|RotateToTarget) 0.016667 true true))
    (Variables|Default|SetLockonTimer _returnvalue_5)))

(event Custom|RotateToTarget
  (bind _lockontarget (Variables|Default|GetLockonTarget))
  (bind _returnvalue (Transformation|GetActorLocation _lockontarget))
  (bind (_x _y _z) (Math|Vector|BreakVector _returnvalue))
  ;[0 1 0 0.5] Start Lockon
  (Utilities|IsValid _lockontarget
    (:Is%20Valid
      (Pawn|SetControlRotation (Game|GetPlayerController 0) (Math|Rotator|FindLookatRotation (Transformation|GetActorLocation (Game|GetPlayerCharacter 0)) (Math|Vector|MakeVector _x _y (- _z 1e+02)))))
    (:Is%20Not%20Valid
      (CallFunction|EndLockon))))

(event Custom|EndLockon
  (bind _returnvalue (Game|GetPlayerCharacter 0))
  (bind _charactermovement (Variables|/Script/Engine.Character|GetCharacterMovement _returnvalue))
  ;[0 1 0 0.5] End Lockon
  (Utilities|Time|ClearandInvalidateTimerbyHandle (Variables|Default|GetLockonTimer))
  (Input|SetIgnoreLookInput (Game|GetPlayerController 0) false)
  (Variables|Default|SetIsLockedon false)
  (Variables|/Script/Engine.SpringArmComponent|SetTargetOffset (Actor|GetComponentbyClass (Components|GetOwner) "/Script/Engine.SpringArmComponent") "0, 0, 0")
  (Variables|/Script/Engine.CharacterMovementComponent|SetbOrientRotationToMovement _charactermovement true)
  (Variables|/Script/Engine.CharacterMovementComponent|SetbUseControllerDesiredRotation _charactermovement false))

(event Custom|DecideLockon
  ;[0 1 0 0.5] Decide Lockon
  (if (Variables|Default|GetIsLockedon)
    (CallFunction|EndLockon)
    (else
      (CallFunction|StartLockon))))