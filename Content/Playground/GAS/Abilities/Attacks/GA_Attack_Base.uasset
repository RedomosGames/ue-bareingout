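; Base Gameplay Ability for melee attacks that checks an attribute can cover AttackCost, then applies it through a SetByCaller cost effect.
; It plays a montage, starts CombatComponent attack rotation and listens for gameplay events.
; Trace events start and stop hand/foot damage traces; Combo events add and remove loose tags, with Combo.End also ending the ability.
; Montage completion or interruption ends it too, and OnEndAbility stops rotation and tracing.
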(event Ability|EventActivateAbility
  (if (<= (* (Variables|Default|GetAttackCost) -1.0) (.ReturnValue (Ability|Attribute|GetFloatAttributefromAbilitySystemComponent (Ability|GetAbilitySystemComponent (Ability|GetAvatarActorfromActorInfo)) "(AttributeName=\"Stamina\",Attribute=/Script/Playground.BasicAttributeSet:Stamina,AttributeOwner=\"/Script/CoreUObject.Class'/Script/Playground.BasicAttributeSet'\")")))
    (bind _returnvalue (Spec|MakeSpecHandle(ByClass) "/Game/Playground/GAS/Effects/GE_Attack_Cost.GE_Attack_Cost_C" 0))
    (bind _returnvalue_2 (Ability|GameplayEffect|AssignTagSetbyCallerMagnitude _returnvalue "(TagName=\"GameplayEffect.Data.AttackCost\")" (Variables|Default|GetAttackCost)))
    (Ability|ApplyGameplayEffectSpecToOwner _returnvalue_2)
    (Variables|Default|SetCombatComp (Actor|GetComponentbyClass (Ability|GetAvatarActorfromActorInfo) "/Game/Playground/Blueprints/Components/CombatComponent.CombatComponent_C"))
    (|PlayMontageandWaitProxy "None" (Variables|Default|GetMontageToPlay) 1.0 "None" true 1.0 0.0 true
      (:then
        (Default|StartAttackRotation (Variables|Default|GetCombatComp))
        (Ability|Tasks|WaitGameplayEvent "(TagName=\"Event.Trace.Start\")" 0
          (:then
            (Ability|Tasks|WaitGameplayEvent "(TagName=\"Event.Trace.End\")" 0
              (:then
                (Ability|Tasks|WaitGameplayEvent "(TagName=\"Event.Combo.Start\")" 0
                  (:then
                    (Ability|Tasks|WaitGameplayEvent "(TagName=\"Event.Combo.End\")" 0
                      (:EventReceived
                        (Ability|GameplayEffect|RemoveLooseGameplayTags (Ability|GetAvatarActorfromActorInfo) (GameplayTags|MakeLiteralGameplayTagContainer (Variables|Default|GetRemoveLooseTag)))
                        (Ability|EndAbility))))
                  (:EventReceived
                    (Ability|GameplayEffect|AddLooseGameplayTags (Ability|GetAvatarActorfromActorInfo) (GameplayTags|MakeLiteralGameplayTagContainer (Variables|Default|GetAddLooseTag))))))
              (:EventReceived
                (Default|TraceEnd (Variables|Default|GetCombatComp)))))
          (:EventReceived
            (Default|StartTrace (Variables|Default|GetCombatComp) (Variables|Default|GetLeft%20Hand%20Trace) (Variables|Default|GetRight%20Hand%20Trace) (Variables|Default|GetLeft%20Foot%20Trace) (Variables|Default|GetRight%20Foot%20Trace) (Variables|Default|GetDamage%20Info)))))
      (:OnCompleted
        (Ability|EndAbility :!label _label))
      (:OnInterrupted
        (goto _label))
      (:OnCancelled
        (goto _label)))
    (else
      (Ability|EndAbility))))

(event Ability|EventOnEndAbility
  (params (bWasCancelled :type Boolean))
  (bind _combatcomp (Variables|Default|GetCombatComp))
  (bind _combatcomp_2 (Variables|Default|GetCombatComp))
  (Utilities|IsValid _combatcomp_2
    (:Is%20Valid
      (Default|EndAttackRotation _combatcomp_2))
    (:Is%20Not%20Valid
      _))
  (Utilities|IsValid _combatcomp
    (:Is%20Valid
      (Default|TraceEnd _combatcomp))))