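; Gameplay ability that knocks the avatar backward as a hit reaction when activated from a gameplay event.
; It rotates the avatar to face its DamageComponent's damage causer, then applies constant root motion force along the reversed forward vector.
; Knockback strength and duration are carried in the event target data's hit result Distance and Time fields.
; On finish, velocity is clamped to the pawn's max movement speed, with a fallback for non-pawns, and the ability ends.
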(event Ability|EventOnEndAbility
  (params (bWasCancelled :type Boolean)))

(event Ability|EventActivateAbilityFromEvent
  (params (EventData :type Gameplay%20Event%20Data%20Structure%20%28by%20ref%29))
  (bind _targetdata (Utilities|Struct|BreakGameplayEventData EventData))
  (bind _returnvalue (Ability|GetAvatarActorfromActorInfo))
  (bind _returnvalue_2 (Ability|TargetData|GetHitResultfromTargetData _targetdata))
  (bind (_bblockinghit _binitialoverlap _time _distance) (Collision|BreakHitResult _returnvalue_2))
  (Transformation|SetActorRotation _returnvalue (Math|Rotator|FindLookatRotation (Transformation|GetActorLocation (Ability|GetAvatarActorfromActorInfo)) (Transformation|GetActorLocation (Variables|/Game/Playground/Blueprints/Components/DamageComponent.DamageComponent_C|GetDamageCauser (Actor|GetComponentbyClass (Ability|GetAvatarActorfromActorInfo) "/Game/Playground/Blueprints/Components/DamageComponent.DamageComponent_C")))))
  (Ability|Tasks|ApplyRootMotionConstantForce "None" (* (Transformation|GetActorForwardVector _returnvalue) -1.0) _distance _time false 0 "ClampVelocity" "0, 0, 0" (CallFunction|GetMovementSpeed)
    (:OnFinish
      (Ability|EndAbility))))

(fn GetMovementSpeed
  (bind _aspawn (Utilities|Casting|CastToPawn (Ability|GetAvatarActorfromActorInfo))
    (:then
      (return (Class|MovementComponent|GetMaxSpeed (Pawn|GetMovementComponent _aspawn))))
    (:CastFailed
      (return 6e+02))))