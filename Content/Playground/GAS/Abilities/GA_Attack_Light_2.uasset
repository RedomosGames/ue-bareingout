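; GA_Attack_Light_2 is the Gameplay Ability for a light attack, playing a montage while the CombatComponent handles attack rotation.
; Gameplay events start and end a left-hand damage trace on that component.
; Combo events swap the loose ComboWindow.1 tag for ComboWindow.2, then remove it and end the ability.
; The ability also ends when the montage completes, is interrupted or is cancelled, and ending it stops attack rotation.
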(event Ability|EventActivateAbility
  (Variables|Default|SetCombatComp (Actor|GetComponentbyClass (Ability|GetAvatarActorfromActorInfo) "/Game/Playground/Blueprints/Components/CombatComponent.CombatComponent_C"))
  (|PlayMontageandWaitProxy "None" (Variables|Default|GetMontage%20to%20Play) 1.0 "None" true 1.0 0.0 true
    (:then
      (Default|StartAttackRotation (Variables|Default|GetCombatComp))
      (Ability|Tasks|WaitGameplayEvent "(TagName=\"Event.Trace.Start\")" 0
        (:then
          (Ability|Tasks|WaitGameplayEvent "(TagName=\"Event.Trace.End\")" 0
            (:then
              (Ability|Tasks|WaitGameplayEvent "(TagName=\"Event.Combo.Start\")" 0
                (:then
                  (Ability|Tasks|WaitGameplayEvent "(TagName=\"Event.Combo.End\")" 0
                    (:EventReceived
                      (Ability|GameplayEffect|RemoveLooseGameplayTags (Ability|GetAvatarActorfromActorInfo) (GameplayTags|MakeLiteralGameplayTagContainer "(GameplayTags=((TagName=\"ComboWindow.2\")))"))
                      (Ability|EndAbility))))
                (:EventReceived
                  (Ability|GameplayEffect|RemoveLooseGameplayTags (Ability|GetAvatarActorfromActorInfo) (GameplayTags|MakeLiteralGameplayTagContainer "(GameplayTags=((TagName=\"ComboWindow.1\")))"))
                  (Ability|GameplayEffect|AddLooseGameplayTags (Ability|GetAvatarActorfromActorInfo) (GameplayTags|MakeLiteralGameplayTagContainer "(GameplayTags=((TagName=\"ComboWindow.2\")))")))))
            (:EventReceived
              (Default|TraceEnd (Variables|Default|GetCombatComp)))))
        (:EventReceived
          (Default|StartTrace (Variables|Default|GetCombatComp) true false false false (Utilities|Struct|MakeS_DamageInfo -1e+01 "NewEnumerator0")))))
    (:OnCompleted
      (Ability|EndAbility :!label _label))
    (:OnInterrupted
      (goto _label))
    (:OnCancelled
      (goto _label))))

(event Ability|EventOnEndAbility
  (params (bWasCancelled :type Boolean))
  (Default|EndAttackRotation (Variables|Default|GetCombatComp)))