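; Dash gameplay ability that propels the avatar along its last movement input, or facing direction when there is none, while hiding its mesh.
; A root motion constant force task drives the burst, clamping exit velocity to the pawn's max speed.
; Activation commits cost, applies a SetByCaller cooldown effect and adds a dash GameplayCue.
; Ending restores mesh visibility and also commits the cooldown.
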(event Ability|EventActivateAbility
  (CallFunction|SetMeshVisiblity false)
  (Ability|CommitAbilityCost false)
  (Ability|Tasks|ApplyRootMotionConstantForce "None" (CallFunction|GetMovementDirection) 1.75e+03 0.3 false 0 "ClampVelocity" "0, 0, 0" (CallFunction|GetMovementSpeed)
    (:then
      (bind _returnvalue (Spec|MakeSpecHandle(ByClass) "/Game/Playground/GAS/Effects/GE_Dash_Cooldown.GE_Dash_Cooldown_C" 0))
      (bind _returnvalue_2 (Ability|GameplayEffect|AssignTagSetbyCallerMagnitude _returnvalue "(TagName=\"GameplayEffect.Data.DashCooldown\")" 2.0))
      (Ability|ApplyGameplayEffectSpecToOwner _returnvalue_2)
      (GameplayCue|AddGameplayCue :GameplayCueTag "(TagName=\"GameplayCue.Dash\")"))
    (:OnFinish
      (Ability|EndAbility))))

(event Ability|EventOnEndAbility
  (params (bWasCancelled :type Boolean))
  (CallFunction|SetMeshVisiblity true)
  (Ability|CommitAbilityCooldown false))

(fn GetMovementDirection
  (bind _aspawn (Utilities|Casting|CastToPawn (Ability|GetAvatarActorfromActorInfo)))
  (if (Math|Vector|VectorIsZero (Class|Pawn|GetLastMovementInputVector _aspawn))
    (return (Transformation|GetActorForwardVector _aspawn))
    (else
      (return (Class|Pawn|GetLastMovementInputVector _aspawn)))))

(fn GetMovementSpeed
  (bind _aspawn (Utilities|Casting|CastToPawn (Ability|GetAvatarActorfromActorInfo))
    (:then
      (return (Class|MovementComponent|GetMaxSpeed (Pawn|GetMovementComponent _aspawn))))
    (:CastFailed
      (return 6e+02))))

(fn SetMeshVisiblity
  (params (IsVisible :type Boolean))
  (bind _ascharacter (Utilities|Casting|CastToCharacter (Ability|GetAvatarActorfromActorInfo)))
  (Rendering|SetVisibility (Variables|/Script/Engine.Character|GetMesh _ascharacter) IsVisible true)
  (return))